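; BP_Puzzle_Master2 is a rotating photo-frame piece for Level 1's second puzzle.
; Interact turns the pivot 90 degrees via timeline with a sound, cycles FramePosition, and sets Finalized by comparing the upcoming position to PuzzleAnswer.
; Each instance polls all instances on a looping timer, stopping and calling the EVDPuzzle2Completed dispatcher once all are finalized.
; Tick prints position and finalized state for debugging.
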(event Custom|RotatePhotoFrame
  ;[0.15 0.15 0.15 0.5] Rotate
  (if (not (Variables|Default|GetFrame%20Moving))
    (Variables|Default|SetFrame%20Moving true)
    (Audio|PlaySound2D "/Game/ZH_Assets/SFX/move_object_sound.move_object_sound" 1.0 1.0 0.0 0 0)
    (bind _alpha (Timeline|Timeline PlayFromStart)
      (:Update
        (Transformation|SetRelativeRotation (Variables|Default|GetPivot) (Math|Rotator|MakeRotator 0.0 (Math|Float|Lerp (.pitch (Variables|Default|GetStarting%20Rotation%20Frame)) (- (.pitch (Variables|Default|GetStarting%20Rotation%20Frame)) 9e+01) _alpha) 0.0) false false))
      (:Finished
        (Variables|Default|SetStarting%20Rotation%20Frame (Math|Rotator|MakeRotator 0.0 (Math|Float|Lerp (.pitch (Variables|Default|GetStarting%20Rotation%20Frame)) (- (.pitch (Variables|Default|GetStarting%20Rotation%20Frame)) 9e+01) _alpha) 0.0))
        (Variables|Default|SetFrame%20Moving false)
        (bind _result (Math|Integer|IncrementInt (Variables|Default|GetFramePosition))
          (:%20%20
            (bind _output_get (Variables|Default|SetFramePosition _result))
            (if (> _output_get 3)
              (Variables|Default|SetFramePosition 0))))))))

(event Custom|PuzzleCheck
  (Variables|Default|SetPuzzleSolved true)
  (for _array_element (Variables|Default|GetNewVar)
    (if (not (Variables|BP_Puzzle_Master2_C|GetFinalized _array_element))
      (Variables|Default|SetPuzzleSolved false)))
  (if (Variables|Default|GetPuzzleSolved)
    (Utilities|Time|ClearandInvalidateTimerbyHandle (stale EventBeginPlay _returnvalue))
    (Default|CallEVDPuzzle2Completed)))

(event EventInteract
  (if (== (+ (Variables|Default|GetFramePosition) 1) (Variables|Default|GetPuzzleAnswer))
    (Variables|Default|SetFinalized true)
    (CallFunction|RotatePhotoFrame)
    (else
      (Variables|Default|SetFinalized false)
      (CallFunction|RotatePhotoFrame))))

(event EventBeginPlay
  (Variables|Default|SetStarting%20Rotation%20Frame (Variables|/Script/Engine.SceneComponent|GetRelativeRotation (Variables|Default|GetPivot)))
  (bind _outactors (Actor|GetAllActorsOfClass "BP_Puzzle_Master2_C"))
  (Variables|Default|SetNewVar _outactors)
  (bind _returnvalue (Utilities|Time|SetTimerbyEvent (delegate Custom|PuzzleCheck) 0.25 true)))

(event EventTick
  (params (DeltaSeconds :type Float%20%28single-precision%29))
  (Development|PrintString (Utilities|String|ToString(Integer) (Variables|Default|GetFramePosition)) true true "(R=0.000000,G=0.660000,B=1.000000,A=1.000000)" DeltaSeconds)
  (Development|PrintString (Utilities|String|ToString(Boolean) (Variables|Default|GetFinalized)) true true "(R=0.000000,G=0.660000,B=1.000000,A=1.000000)" DeltaSeconds))

(fn ConstructionScript
  (|CallParentFunction))