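; Interactive hinged door that opens away from the player, supports key locking and can close itself.
; Interact toggles the door; when locked, it compares only the last player key with its ID, then unlocks and opens or shakes.
; A dot product picks the swing side for a timeline-driven hinge rotation, reversed to close, with sounds.
; Optional auto-close uses a looping timer to shut the door beyond a set player distance.
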(event Custom|ShakeDoor
  (bind _alpha (Timeline|TL_ShakeDoor PlayFromStart)
    (:Update
      (Transformation|SetRelativeRotation (Variables|Default|GetDoorHin) (Math|Rotator|MakeRotator 0.0 0.0 _alpha) false false))))

(event Custom|OpenCloseDoor
  (bind _self self)
  ;[0.15 0.15 0.15 0.5] OpenClose Logic
  (CallFunction|Sounds)
  (if (Variables|Default|GetDoorClosed?)
    (Variables|Default|SetDoorClosed? false)
    (Variables|Default|SetDotProduct (Math|Vector|DotProduct (Math|Vector|Normalize (- (Transformation|GetActorLocation _self) (Transformation|GetActorLocation (Variables|Default|GetPlayerRef)))) (Transformation|GetActorRightVector _self)))
    (bind _door (Timeline|TL_OpenDoor Play)
      (:Update
        (Transformation|SetRelativeRotation (Variables|Default|GetDoorHin) (Math|Rotator|MakeRotator 0.0 0.0 (Math|Float|Lerp 0.0 (Math|Float|SelectFloat 9e+01 -9e+01 (>= (Variables|Default|GetDotProduct) 0.0)) _door)) false false)))
    (else
      (Variables|Default|SetDoorClosed? true)
      (Timeline|TL_OpenDoor Reverse))))

(event Custom|AutoClose
  ;[0.15 0.15 0.15 0.5] Auto Close Door
  (if (Variables|Default|GetAutoClose?)
    (Utilities|Time|SetTimerbyEvent (delegate Custom|DoorAutoClose) 1.0 true)))

(event Custom|DoorAutoClose
  ;[0.15 0.15 0.15 0.5] Auto Close Door
  (if (not (Variables|Default|GetDoorClosed?))
    (if (> (Math|Vector|Distance(Vector) (Transformation|GetActorLocation (Variables|Default|GetPlayerRef)) (Transformation|GetActorLocation)) (Variables|Default|GetClose%20Distance))
      (CallFunction|OpenCloseDoor))))

(event Custom|CheckForKey
  (bind _playerref (Variables|Default|GetPlayerRef))
  ;[0.15 0.15 0.15 0.5] KeyCheck
  (for _array_element (Variables|/Game/FirstPerson/Blueprints/BP_FirstPersonCharacter.BP_FirstPersonCharacter_C|GetKeys _playerref)
    _)
  (if (Utilities|Enum|Equal(Enum) _array_element (Variables|Default|GetDoorKeyID))
    (CallFunction|UnlockDoor)
    (Variables|/Game/FirstPerson/Blueprints/BP_FirstPersonCharacter.BP_FirstPersonCharacter_C|SetHasKey? _playerref false)
    (else
      (CallFunction|ShakeDoor))))

(event Custom|UnlockDoor
  ;[0.15 0.15 0.15 0.5] UnlockDoor
  (Variables|Default|SetLocked? false)
  (Audio|PlaySoundatLocation (Variables|Default|GetUnlock%20Sound) (Transformation|GetWorldLocation (Variables|Default|GetDoorHin)) "0, 0, 0" 1.0 1.0 0.0 0 0 0 0)
  (CallFunction|OpenCloseDoor))

(event EventBeginPlay
  (bind _asbp_first_person_character (Utilities|Casting|CastToBP_FirstPersonCharacter (Game|GetPlayerCharacter 0)))
  (Variables|Default|SetPlayerRef _asbp_first_person_character)
  (CallFunction|AutoClose))

(event EventInteract
  ;[0.15 0.15 0.15 0.5] Interaction
  (if (Variables|Default|GetLocked?)
    (CallFunction|CheckforKey)
    (else
      (CallFunction|OpenCloseDoor))))

(fn ConstructionScript)

(fn Sounds
  (bind _door3 (Variables|Default|Getdoor3))
  (bind _returnvalue (Transformation|GetWorldLocation _door3))
  (if (Variables|Default|GetLocked?)
    (Audio|PlaySoundatLocation (Variables|Default|GetLockSound) _returnvalue "0, 0, 0" 1.0 1.0 0.0 0 0 0 0)
    (elif (Variables|Default|GetDoorClosed?)
      (Audio|PlaySoundatLocation (Variables|Default|GetOpenSound) _returnvalue "0, 0, 0" 1.0 1.0 0.0 0 0 0 0)
      (else
        (Audio|PlaySoundatLocation (Variables|Default|GetCloseSound) _returnvalue "0, 0, 0" 1.0 1.0 0.0 0 0 0 0)))))