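; Door actor that slides and/or rotates its hinge, toggled by Interact or character overlap unless locked.
; Both paths share a FlipFlop that plays or reverses a timeline lerping the hinge transform, with a multicast sound.
; Overlap calls a server toggle when the first character enters the box; the exit count check never passes, so leaving does not close it.
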(event Custom|Mulicast_FX
  (Audio|PlaySoundatLocation (Variables|Default|GetDoor%20Sound) (Transformation|GetActorLocation) "0, 0, 0" 1.0 1.0 0.0 0 0 0 0))

(event Custom|Server_ToggleDoor
  (if (CallFunction|IsLocked (Variables|Default|GetCanOverlap))
    (CallFunction|MulicastFX)
    (Utilities|FlowControl|FlipFlop
      (:A
        (bind _alpha (Timeline|TL_Door Play)
          (:Update
            (CallFunction|DoorTransform _alpha))))
      (:B
        (Timeline|TL_Door Reverse)))))

(event EventInteract
  (if (CallFunction|IsLocked (Variables|Default|GetCanInteract))
    (CallFunction|MulicastFX)
    (Utilities|FlowControl|FlipFlop
      (:A
        (bind _alpha (Timeline|TL_Door Play)
          (:Update
            (CallFunction|DoorTransform _alpha))))
      (:B
        (Timeline|TL_Door Reverse)))))

(event Collision|EventActorBeginOverlap
  (params (OtherActor :type Actor%20Object%20Reference))
  (CallFunction|ToggleOverlapDoor OtherActor true))

(event Collision|EventActorEndOverlap
  (params (OtherActor :type Actor%20Object%20Reference))
  (CallFunction|ToggleOverlapDoor OtherActor false))

(fn ConstructionScript)

(fn IsLocked
  (params (Action :type Boolean))
  (return (and Action (not (Variables|Default|GetLocked)))))

(fn DoorTransform
  (params (Alpha :type Float%20%28double-precision%29))
  (Transformation|SetRelativeTransform (Variables|Default|GetDoorHin) (Math|Transform|Lerp(Transform) (Math|Transform|MakeTransform "0, 0, 0") (Math|Transform|MakeTransform (Variables|Default|GetSlide%20Rotation) (Variables|Default|GetRotation%20Amount) "1.000000,1.000000,1.000000") Alpha "EulerInterp") false false))

(fn ToggleOverlapDoor
  (params (Player :type Object%20Object%20Reference) (On :type Boolean))
  (bind _box (Variables|Default|GetBox))
  (bind _overlappingactors (Collision|GetOverlappingActors _box "/Script/Engine.Character" :!class /Script/Engine.PrimitiveComponent))
  (bind _returnvalue (Utilities|Array|Length _overlappingactors))
  (Utilities|Casting|CastToCharacter Player)
  (if (select On (not (> _returnvalue 1)) (not (>= _returnvalue 0)))
    (CallFunction|ServerToggleDoor)))