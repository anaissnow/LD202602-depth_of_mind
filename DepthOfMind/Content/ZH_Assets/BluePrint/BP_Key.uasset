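; BP_Key is a pickup key actor that the player collects through interaction.
; On BeginPlay it caches the player character as BP_ThirdPersonCharacter.
; Its Interact event plays a grab sound, adds its KeyID to the player's keys, and destroys itself.
; The construction script applies the configurable KeyMesh to its static mesh component.
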(event EventBeginPlay
  (bind _asbp_third_person_character (Utilities|Casting|CastToBP_ThirdPersonCharacter (Game|GetPlayerCharacter 0)))
  (Variables|Default|SetPlayer%20Ref _asbp_third_person_character))

(event EventInteract
  (Audio|PlaySound2D "/Game/ZH_Assets/SFX/grab_key.grab_key" 1.0 1.0 0.0 0 0)
  (Default|AddKeys (Variables|Default|GetPlayer%20Ref) (Variables|Default|GetKey%20ID))
  (Actor|DestroyActor))

(fn ConstructionScript
  (Components|StaticMesh|SetStaticMesh (Variables|Default|GetStaticMesh) (Variables|Default|Getkey%20mesh)))