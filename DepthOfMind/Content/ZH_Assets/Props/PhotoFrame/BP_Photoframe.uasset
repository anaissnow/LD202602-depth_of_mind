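; BP_Photoframe is an interactable photo frame prop that the player can rotate in fixed steps.
; Overlapping InteractBox with BP_ThirdPersonCharacter enables interaction and shows a prompt widget created at BeginPlay; leaving disables it and removes the prompt.
; Each Interact event, while enabled, instantly adds a local rotation increment to the Pivot component, with no animation or limit.
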(event OnComponentBeginOverlap(InteractBox)
  (params (OverlappedComponent :type Primitive%20Component%20Object%20Reference) (OtherActor :type Actor%20Object%20Reference) (OtherComp :type Primitive%20Component%20Object%20Reference) (OtherBodyIndex :type Integer) (bFromSweep :type Boolean) (SweepResult :type Hit%20Result%20Structure%20%28by%20ref%29))
  (Utilities|Casting|CastToBP_ThirdPersonCharacter OtherActor)
  (Variables|Default|Setcan%20interact true)
  (UserInterface|Viewport|AddtoViewport (Variables|Default|GetInteract%20Prompt) 0))

(event OnComponentEndOverlap(InteractBox)
  (params (OverlappedComponent :type Primitive%20Component%20Object%20Reference) (OtherActor :type Actor%20Object%20Reference) (OtherComp :type Primitive%20Component%20Object%20Reference) (OtherBodyIndex :type Integer))
  (Utilities|Casting|CastToBP_ThirdPersonCharacter OtherActor)
  (Variables|Default|Setcan%20interact false)
  (Widget|RemovefromParent (Variables|Default|GetInteract%20Prompt)))

(event EventBeginPlay
  (bind _returnvalue (UserInterface|CreateWidget "/Game/ZH_Assets/BluePrint/Prompt_Interface.Prompt_Interface_C"))
  (Variables|Default|SetInteract%20Prompt _returnvalue))

(event EventInteract
  (if (Variables|Default|Getcan%20interact)
    (Transformation|AddLocalRotation (Variables|Default|GetPivot) "45.000000,0.000000,0.000000" false false)))

(fn ConstructionScript)